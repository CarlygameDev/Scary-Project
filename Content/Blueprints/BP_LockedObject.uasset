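; BP_LockedObject is a locked object whose door opens when given the matching item name.
; Open prints a debug string, compares the passed ObjectName with UnlockItemName, and on a match snaps Door to a fixed world rotation and returns the result.
; The event graph holds an unconnected copy of this logic that never runs, and the construction script is empty.
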(fn `Open`
  (params (`Object Name` :type String))
  (returns (`is Correct Key` :type Boolean))
  (bind _returnvalue (`KismetStringLibrary.EqualEqual_StrStr` `Object Name` (`self.Unlock item name`)))
  (`KismetSystemLibrary.PrintString` "Hello")
  (if _returnvalue
    (`SceneComponent.K2_SetWorldRotation` (`self.door`) (struct :`Yaw` 200.0) false false)
    (return _returnvalue)))

(fn `UserConstructionScript`)