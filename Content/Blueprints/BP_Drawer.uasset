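; BP_Drawer is an interactable drawer with a door that the player can get into and out of.
; Each Interact call toggles the Inside flag and teleports player 0 to the location and rotation of the RefInside or RefOutside component.
; The Door snaps to a fixed yaw for each state, with no animation.
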(event `/Game/Blueprints/BPI_Interaction.Interact`
  (bind (_returnvalue_location _returnvalue_rotation) (`KismetMathLibrary.BreakTransform` (`SceneComponent.K2_GetComponentToWorld` (`self.ref inside`))))
  (bind (_returnvalue_location_2 _returnvalue_rotation_2) (`KismetMathLibrary.BreakTransform` (`SceneComponent.K2_GetComponentToWorld` (`self.ref  outside`))))
  (if (not (`self.inside`))
    (set `self.inside` true)
    (`self.K2_SetActorTransform` (`GameplayStatics.GetPlayerCharacter` 0) (`KismetMathLibrary.MakeTransform` _returnvalue_location _returnvalue_rotation) false false)
    (`SceneComponent.K2_SetRelativeRotation` (`self.door`) (struct :`Yaw` 40.0) false false)
    (else
      (set `self.inside` false)
      (`self.K2_SetActorTransform` (`GameplayStatics.GetPlayerCharacter` 0) (`KismetMathLibrary.MakeTransform` _returnvalue_location_2 _returnvalue_rotation_2) false false)
      (`SceneComponent.K2_SetRelativeRotation` (`self.door`) (struct :`Yaw` 172.0) false false))))

(fn `UserConstructionScript`)